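; Player tank Blueprint that registers its barrel and provides an orbiting camera.
; On BeginPlay it passes the TankBarrel component to SetBarrelReference, which is defined outside these graphs.
; Azimut and Elevation axis inputs yaw a gimbal and pitch the spring arm separately, scaled by delta time and CameraRotationSpeed for frame-rate independent rotation.
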(event EventBeginPlay
  (Class|Tank|SetBarrelReference (Variables|Default|GetTankBarrel)))

(event Input|AxisEvents|InputAxisAzimut
  (params (AxisValue :type Float%20%28single-precision%29))
  (Transformation|AddLocalRotation (Variables|Default|GetAzimutGimbal) (Math|Rotator|MakeRotator 0.0 0.0 (* AxisValue (Utilities|Time|GetWorldDeltaSeconds) (Variables|Default|GetCameraRotationSpeed))) false false))

(event Input|AxisEvents|InputAxisElevation
  (params (AxisValue :type Float%20%28single-precision%29))
  (Transformation|AddLocalRotation (Variables|Default|GetSpringArm) (Math|Rotator|MakeRotator 0.0 (* AxisValue (Utilities|Time|GetWorldDeltaSeconds) (Variables|Default|GetCameraRotationSpeed)) 0.0) false false))

(fn ConstructionScript)